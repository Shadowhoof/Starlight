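; BP_StarlightCharacter is the player character for Starlight, adding a HUD on BeginPlay and hard-wired debug keys for physics and portal testing.
; SpaceBar launches a BP_Cube_02 from the camera with a velocity-change impulse, and B has PortalComponent debug-spawn the same cube class in a portal.
; V line-traces from the eye viewpoint and shoves the hit component along the actor's forward vector rather than the view direction.
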(event `self.ReceiveBeginPlay`
  (bind _returnvalue (`|CreateWidget` "/Game/Starlight/UI/WBP_HUD.WBP_HUD_C" (`GameplayStatics.GetPlayerController` 0)))
  (`UserWidget.AddToViewport` _returnvalue 0))

(event `self.ReceiveTick`
  (params (DeltaSeconds :type "Float (single-precision)")))

(event `Key|SpaceBar`
  (params (Key :type "Key Structure"))
  (bind _cameracomponent (`self.CameraComponent`))
  (bind _returnvalue (`SceneComponent.K2_GetComponentRotation` _cameracomponent))
  ;[1 1 1] Debug throw cube
  (:`Pressed`
    (bind _returnvalue_2 (`|SpawnActorFromClass` "/Game/Starlight/Props/Blueprints/BP_Cube_02.BP_Cube_02_C" (`KismetMathLibrary.MakeTransform` (+ (`SceneComponent.K2_GetComponentLocation` _cameracomponent) (* (`KismetMathLibrary.GetForwardVector` _returnvalue) 50.0)) _returnvalue) "AlwaysSpawn" "OverrideRootScale" self self))
    (`PrimitiveComponent.AddImpulse` (`StarlightActor.MeshComponent` _returnvalue_2) (* (`KismetMathLibrary.GetForwardVector` (`SceneComponent.K2_GetComponentRotation` (`self.CameraComponent`))) 1000.0) "None" true)))

(event `Key|B`
  (params (Key :type "Key Structure"))
  (:`Pressed`
    (`PortalComponent.DebugSpawnObjectInPortal` (`self.PortalComponent`) "/Game/Starlight/Props/Blueprints/BP_Cube_02.BP_Cube_02_C")))

(event `Key|V`
  (params (Key :type "Key Structure"))
  (bind (_outlocation _outrotation) (`self.GetActorEyesViewPoint`))
  (:`Pressed`
    (bind _outhit (`KismetSystemLibrary.LineTraceSingle` _outlocation (+ _outlocation (* (`KismetMathLibrary.GetForwardVector` _outrotation) 10000.0)) "TraceTypeQuery1"))
    (`PrimitiveComponent.AddImpulse` (`.HitComponent` (`GameplayStatics.BreakHitResult` _outhit)) (* (`self.GetActorForwardVector`) 300000.0) "None" false)))

(fn `UserConstructionScript`)